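; BP_GridManager builds the visual battlefield grid in its construction script, with spawn zones for two players.
; Grid lines are scaled cube meshes and cells are plane meshes, both sized from grid dimensions and cell size and toggled independently.
; Each cell's material marks Player 1, Player 2 or neutral ground by its Y row.
; Existing visuals are cleared first, and map boundaries regenerate whenever either layer is shown.
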(event EventBeginPlay)

(event Collision|EventActorBeginOverlap
  (params (OtherActor :type Actor%20Object%20Reference)))

(event EventTick
  (params (DeltaSeconds :type Float%20%28single-precision%29)))

(fn ConstructionScript
  (Class|GridManager|ClearGridVisuals)
  (if (Variables|Default|GetbShowGrid)
    (CallFunction|GenerateGridLines)
    (if (Variables|Components|GridVisual|GetShowCellTextures)
      (CallFunction|GenerateCellTextures)
      (Class|GridManager|RegenerateMapBoundaries)
      (else
        (Class|GridManager|RegenerateMapBoundaries)))
    (elif (Variables|Components|GridVisual|GetShowCellTextures)
      (CallFunction|GenerateCellTextures)
      (Class|GridManager|RegenerateMapBoundaries))))

(fn GenerateGridLines
  (bind _cellsize (Variables|Default|GetCellSize))
  (bind _cellsize_2 (Variables|Default|GetCellSize))
  (for _index (range 0 (Variables|Default|GetGridWidth))
    (bind _returnvalue (AddComponent|AddStaticMeshComponent false))
    (Class|GridManager|AddGridLineComponent _returnvalue)
    (Variables|Default|SetNewVerticalLine _returnvalue)
    (Components|StaticMesh|SetStaticMesh (Variables|Default|GetNewVerticalLine) "/Engine/BasicShapes/Cube.Cube")
    (Transformation|SetRelativeLocation (Variables|Default|GetNewVerticalLine) (Math|Vector|MakeVector (* _index _cellsize_2) (/ (* _cellsize_2 (Variables|Default|GetGridHeight)) 2.0) 1.0) false false)
    (Transformation|SetRelativeScale3D (Variables|Default|GetNewVerticalLine) (Math|Vector|MakeVector (/ (Variables|Default|GetLineThickness) 1e+02) (/ (* (Variables|Default|GetGridHeight) _cellsize_2) 1e+02) 0.01))
    (Rendering|Material|SetMaterial (Variables|Default|GetNewVerticalLine) 0 (Variables|Default|GetGridLineMaterial)))
  (for _index_2 (range 0 (Variables|Default|GetGridHeight))
    (bind _returnvalue_2 (AddComponent|AddStaticMeshComponent false))
    (Class|GridManager|AddGridLineComponent _returnvalue_2)
    (Variables|Default|SetNewVerticalLine _returnvalue_2)
    (Components|StaticMesh|SetStaticMesh (Variables|Default|GetNewVerticalLine) "/Engine/BasicShapes/Cube.Cube")
    (Transformation|SetRelativeLocation (Variables|Default|GetNewVerticalLine) (Math|Vector|MakeVector (/ (* _cellsize (Variables|Default|GetGridWidth)) 2.0) (* _index_2 _cellsize) 1.0) false false)
    (Transformation|SetRelativeScale3D (Variables|Default|GetNewVerticalLine) (Math|Vector|MakeVector (/ (* (Variables|Default|GetGridWidth) _cellsize) 1e+02) (/ (Variables|Default|GetLineThickness) 1e+02) 0.01))
    (Rendering|Material|SetMaterial (Variables|Default|GetNewVerticalLine) 0 (Variables|Default|GetGridLineMaterial))))

(fn GenerateCellTextures
  (bind _cellcomponents_ (Variables|Components|GridVisual|GetCellComponents%20))
  (bind _cellsize (Variables|Default|GetCellSize))
  (bind _cellsize_2 (Variables|Default|GetCellSize))
  (bind _cellsize_3 (Variables|Default|GetCellSize))
  (bind _returnvalue (/ _cellsize 1e+02))
  (for _array_element _cellcomponents_
    (Utilities|IsValid _array_element
      (:Is%20Valid
        (Components|DestroyComponent _array_element))))
  (Utilities|Array|Clear _cellcomponents_)
  (for _index (range 0 (- (Variables|Default|GetGridWidth) 1))
    (for _index_2 (range 0 (- (Variables|Default|GetGridHeight) 1))
      (bind _returnvalue_2 (AddComponent|AddStaticMeshComponent false))
      (Variables|Components|GridVisual|SetNewCell _returnvalue_2)
      (Components|StaticMesh|SetStaticMesh (Variables|Components|GridVisual|GetNewCell) "/Engine/BasicShapes/Plane.Plane")
      (Transformation|SetRelativeLocation (Variables|Components|GridVisual|GetNewCell) (Math|Vector|MakeVector (+ (* (Math|Conversions|ToFloat(Integer) _index) _cellsize_3) (/ _cellsize_3 2.0)) (+ (* (Math|Conversions|ToFloat(Integer) _index_2) _cellsize_2) (/ _cellsize_2 2.0)) 0.1) false false)
      (Transformation|SetRelativeScale3D (Variables|Components|GridVisual|GetNewCell) (Math|Vector|MakeVector _returnvalue _returnvalue 1.0))
      (bind _material (CallFunction|GetMaterialforCell (Math|Vector2D|MakeVector2D (Math|Conversions|ToFloat(Integer) _index) (Math|Conversions|ToFloat(Integer) _index_2))))
      (Rendering|Material|SetMaterial (Variables|Components|GridVisual|GetNewCell) 0 _material)
      (Utilities|Array|Add (Variables|Components|GridVisual|GetCellComponents%20) (Variables|Components|GridVisual|GetNewCell)))))

(fn GetMaterialforCell
  (params (GridPosition :type Vector%202D%20Structure))
  (bind _y (Math|Vector2D|BreakVector2D GridPosition))
  (if (< _y (Math|Conversions|ToFloat(Integer) (Variables|Default|GetPlayer1SpawnSize)))
    (return (Variables|Components|GridVisual|GetCellPlayer1Material))
    (elif (>= _y (Math|Conversions|ToFloat(Integer) (- (Variables|Default|GetGridHeight) (Variables|Default|GetPlayer2SpawnSize))))
      (return (Variables|Components|GridVisual|GetCellPlayer2Material))
      (else
        (return (Variables|Components|GridVisual|GetCellNeutralMaterial))))))