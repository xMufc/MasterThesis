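; Player camera pawn that holds a target height above the ground and supports curve-driven zoom.
; BeginPlay initializes its movement component; each Tick traces straight down to measure ground distance.
; If too high it drops by the exact excess, but if too low it rises by a fixed 290-unit step, without sweeping.
; SetArmLength maps a zoom amount through a float curve to the camera arm length.
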(event EventBeginPlay
  (Default|InitComponent (Variables|Components|GetPawnMovementComponent)))

(event EventTick
  (params (DeltaSeconds :type Float%20%28single-precision%29))
  (Camera|Height|AdjustCameraHeight))

(fn ConstructionScript)

(fn SetArmLength
  (params (InZoomAmount :type Float%20%28double-precision%29))
  (bind _curvezoomarmlength (Variables|Camera|Zoom|GetCurveZoomArmLength)
    (:then
      (Variables|/Script/Engine.SpringArmComponent|SetTargetArmLength (Variables|Components|GetCamera) (Math|Curves|GetFloatValue _curvezoomarmlength InZoomAmount)))
    (:else
      _))
  (return))

(fn AdjustCameraHeight
  (bind _returnvalue (Transformation|GetActorLocation))
  (bind _outhit (Collision|LineTraceByChannel _returnvalue (- _returnvalue "0.000000,0.000000,100000.000000") "TraceTypeQuery3" false 0 "None"))
  (LocalVariables|SetDistanceLocal (Math|Vector|VectorLength (- (.ImpactPoint (Collision|BreakHitResult _outhit)) (Transformation|GetActorLocation))))
  (if (Math|Float|NearlyEqual(Float) (LocalVariables|GetDistanceLocal) (Variables|Default|GetTargetPawnHeight) 0.1)
    _
    (elif (> (LocalVariables|GetDistanceLocal) (Variables|Default|GetTargetPawnHeight))
      (Transformation|SetActorLocation (- (Transformation|GetActorLocation) (Math|Vector|MakeVector 0.0 0.0 (- (LocalVariables|GetDistanceLocal) (Variables|Default|GetTargetPawnHeight)))) false false)
      (else
        (Transformation|SetActorLocation (+ (Transformation|GetActorLocation) (Math|Vector|MakeVector 0.0 0.0 2.9e+02)) false false))))
  (return))