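; Player controller that turns player input into camera control for a BP_CameraPawn, with the mouse cursor shown.
; On BeginPlay it caches the pawn's movement component, which executes all movement, speed modifier, zoom, pan and reset commands.
; Movement axes share one validity-checked call, and mouse movement triggers edge scrolling.
; Holding Pan disables edge scrolling and opens a gate that feeds scaled MouseX into camera panning.
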(event EventBeginPlay
  (Utilities|FlowControl|Sequence
    (:then_0
      (Variables|Default|SetbShowMouseCursor true)
      (bind _asbp_camera_pawn (Utilities|Casting|CastToBP_CameraPawn (Game|Player|GetPlayerPawn 0)))
      (bind _output_get (Variables|References|SetCameraPawnRef _asbp_camera_pawn))
      (Variables|Default|SetCameraMovementRef (Variables|/Game/Core/Player/BP_CameraPawn.BP_CameraPawn_C|GetPawnMovementComponent _output_get)))))

(event EventTick
  (params (DeltaSeconds :type Float%20%28single-precision%29)))

(event Input|ActionEvents|InputActionZoomIn
  (params (Key :type Key%20Structure :default "None"))
  (:Pressed
    (Default|Zoomin (Variables|Default|GetCameraMovementRef))))

(event Input|ActionEvents|InputActionZoomOut
  (params (Key :type Key%20Structure :default "None"))
  (:Pressed
    (Default|ZoomOut (Variables|Default|GetCameraMovementRef))))

(event Input|ActionEvents|InputActionZoomReset
  (params (Key :type Key%20Structure :default "None"))
  (:Pressed
    (Default|ResetZoom (Variables|Default|GetCameraMovementRef))))

(event Input|ActionEvents|InputActionPanReset
  (params (Key :type Key%20Structure :default "None"))
  (:Pressed
    (Default|ResetPan (Variables|Default|GetCameraMovementRef))))

(event Input|ActionEvents|InputActionSpeedModifier
  (params (Key :type Key%20Structure :default "None"))
  (bind _cameramovementref (Variables|Default|GetCameraMovementRef))
  (:Pressed
    (Default|SetSpeedModifier _cameramovementref 2.0))
  (:Released
    (Default|SetSpeedModifier _cameramovementref 1.0)))

(event Input|ActionEvents|InputActionPan
  (params (Key :type Key%20Structure :default "None"))
  (bind _cameramovementref (Variables|Default|GetCameraMovementRef))
  (:Pressed
    (Default|SetDisableEdgeScroll _cameramovementref true)
    (Utilities|FlowControl|Gate true) ; enters at Open
  )
  (:Released
    (Default|SetDisableEdgeScroll _cameramovementref false)
    (Utilities|FlowControl|Gate true) ; enters at Close
  ))

(event Input|ActionEvents|InputActionCameraReset
  (params (Key :type Key%20Structure :default "None"))
  (:Pressed
    (Default|ResetCamera (Variables|Default|GetCameraMovementRef))))

(event Input|AxisEvents|InputAxisMoveForward
  (params (AxisValue :type Float%20%28single-precision%29))
  (Utilities|IsValid (Variables|Default|GetCameraMovementRef)
    (:Is%20Valid
      (Default|BasicMovementController (Variables|Default|GetCameraMovementRef) AxisValue (stale Input|AxisEvents|InputAxisMoveRight AxisValue)))
    (:Is%20Not%20Valid
      (Development|PrintString "Camera Movement Ref - Not Valid" false))))

(event Input|AxisEvents|InputAxisMoveRight
  (params (AxisValue :type Float%20%28single-precision%29))
  (Utilities|IsValid (Variables|Default|GetCameraMovementRef)
    (:Is%20Valid
      (Default|BasicMovementController (Variables|Default|GetCameraMovementRef) (stale Input|AxisEvents|InputAxisMoveForward AxisValue) AxisValue))
    (:Is%20Not%20Valid
      (Development|PrintString "Camera Movement Ref - Not Valid" false))))

(event Input|MouseEvents|MouseX
  (params (AxisValue :type Float%20%28single-precision%29))
  (Utilities|FlowControl|Gate true
    (:Exit
      (Default|PanCamera (Variables|Default|GetCameraMovementRef) (* AxisValue (Variables|Camera|Settings|GetPanSensitivity))))))

(event Input|MouseEvents|MouseX
  (params (AxisValue :type Float%20%28single-precision%29))
  (Utilities|IsValid (Variables|Default|GetCameraMovementRef)
    (:Is%20Valid
      (Default|EdgeScroll (Variables|Default|GetCameraMovementRef)))
    (:Is%20Not%20Valid
      (Development|PrintString "Camera Movement Ref - Not Valid" false))))

(event Input|MouseEvents|MouseY
  (params (AxisValue :type Float%20%28single-precision%29))
  (Utilities|IsValid (Variables|Default|GetCameraMovementRef)
    (:Is%20Valid
      (Default|EdgeScroll (Variables|Default|GetCameraMovementRef)))
    (:Is%20Not%20Valid
      (Development|PrintString "Camera Movement Ref - Not Valid" false))))

(fn ConstructionScript)