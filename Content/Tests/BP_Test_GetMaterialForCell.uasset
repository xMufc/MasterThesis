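; BP_Test_GetMaterialForCell is a functional test that checks the material the grid manager's GetMaterialForCell returns for cells on the grid.
; On StartTest it expects the player 1 material at the origin, the player 2 material at the last row of the first column, and the neutral material near the center.
; Assertions chain in sequence, finishing as succeeded only if all three match, otherwise failed.
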(event EventStartTest
  (bind _gridmanagerref (Variables|Default|GetGridManagerRef))
  (bind _gridmanagerref_2 (Variables|Default|GetGridManagerRef))
  (bind _material (Default|GetMaterialforCell (Variables|Default|GetGridManagerRef)))
  (bind _returnvalue (Class|FunctionalTest|AssertEqualObject _material "/Game/Maps/Materials/CellMaterials/MI_CellPlayer1.MI_CellPlayer1"))
  (if _returnvalue
    (bind _material_2 (Default|GetMaterialforCell _gridmanagerref_2 (Math|Vector2D|MakeVector2D 0.0 (Math|Conversions|ToFloat(Integer) (- (Variables|/Script/MagisterkaBKonkel.GridManager|GetGridHeight _gridmanagerref_2) 1)))))
    (bind _returnvalue_2 (Class|FunctionalTest|AssertEqualObject _material_2 "/Game/Maps/Materials/CellMaterials/MI_CellPlayer2.MI_CellPlayer2"))
    (if _returnvalue_2
      (bind _material_3 (Default|GetMaterialforCell _gridmanagerref (Math|Vector2D|MakeVector2D (Math|Conversions|ToFloat(Integer) (/ (Variables|/Script/MagisterkaBKonkel.GridManager|GetGridHeight _gridmanagerref) 2)) (Math|Conversions|ToFloat(Integer) (/ (Variables|/Script/MagisterkaBKonkel.GridManager|GetGridWidth _gridmanagerref) 2)))))
      (bind _returnvalue_3 (Class|FunctionalTest|AssertEqualObject _material_3 "/Game/Maps/Materials/CellMaterials/M_CellNeutral.M_CellNeutral"))
      (if _returnvalue_3
        (Class|FunctionalTest|FinishTest "Succeeded")
        (else
          (Class|FunctionalTest|FinishTest "Failed" :!label _label)))
      (else
        (goto _label)))
    (else
      (goto _label))))

(fn ConstructionScript)