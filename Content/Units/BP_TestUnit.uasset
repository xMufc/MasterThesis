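; BP_TestUnit is a test unit Blueprint that holds sample nodes and has no working gameplay logic.
; BeginPlay has only an empty branch, while a SetTarget call, a DataTable cast and a CostArmorUnit addition sit disconnected.
; An ArraySum function totals an array's elements in a loop with a local accumulator, and nothing in the file calls it.
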(event EventBeginPlay
  ;[0.15 0.15 0.15 0.5] Przykładowe węzły
  (if true
    _))

(fn ConstructionScript)

(fn ArraySum
  (params (tab :type Array%20of%20Integers))
  (for _index (range 0 (- (Utilities|Array|Length tab) 1))
    (LocalVariables|SetNewLocalVar (+ (Utilities|Array|Get(acopy) tab _index) (LocalVariables|GetNewLocalVar))))
  (return (LocalVariables|GetNewLocalVar)))